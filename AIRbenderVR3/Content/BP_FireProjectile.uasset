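; Fire projectile actor that extends a parent projectile with an explosion on impact.
; Its Apply Damage override runs the parent damage logic, then passes the impact location to a SpawnEmitter event.
; That event spawns a half-scale explosion particle effect at that point and destroys the projectile.
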(event Custom|Spawn%20Emitter
  (params (ImpactLocation :type Vector))
  (Effects|SpawnEmitteratLocation "/Game/FXVarietyPack/Particles/P_ky_explosion.P_ky_explosion" ImpactLocation "0, 0, 0" "0.500000,0.500000,0.500000")
  (Actor|DestroyActor))

(event EventBeginPlay
  (|CallParentFunction) ; This node is disabled and will not be called.\nDrag off pins to build functionality.
)

(event Collision|EventActorBeginOverlap
  (params (OtherActor :type Actor%20Object%20Reference))
  (|CallParentFunction OtherActor) ; This node is disabled and will not be called.\nDrag off pins to build functionality.
)

(event EventTick
  (params (DeltaSeconds :type Float%20%28single-precision%29))
  (|CallParentFunction DeltaSeconds) ; This node is disabled and will not be called.\nDrag off pins to build functionality.
)

(fn ConstructionScript
  (|CallParentFunction))

(fn ApplyDamage
  (params (DamagedActor :type Actor%20Object%20Reference) (ImpactLocationIn :type Vector :default "0, 0, 0"))
  (|CallParentFunction DamagedActor ImpactLocationIn)
  (CallFunction|SpawnEmitter ImpactLocationIn))