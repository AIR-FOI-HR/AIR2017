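; Thunder projectile, a child Blueprint that adds lightning-ball audio and impact effects to its parent projectile's behavior.
; It starts a looping thunder sound on BeginPlay.
; Its Apply Damage override calls the parent, then fires SpawnEmitter, which spawns a half-scale hit particle and impact sound at the impact location, stops the loop and destroys the actor.
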(event Custom|Spawn%20Emitter
  (params (Impact%20Location :type Vector))
  (Effects|SpawnEmitteratLocation "/Game/FXVarietyPack/Particles/P_ky_ThunderBallHit.P_ky_ThunderBallHit" Impact%20Location "0, 0, 0" "0.500000,0.500000,0.500000")
  (Audio|PlaySoundatLocation "/Game/Sounds/A_ThunderHit.A_ThunderHit" Impact%20Location "0, 0, 0" 1.0 1.0 0.0 0 0 0)
  (Components|Activation|Deactivate (Variables|Default|GetAudio))
  (Actor|DestroyActor))

(event EventBeginPlay
  (bind _audio (Variables|Default|GetAudio))
  (|CallParentFunction)
  (Audio|Components|Audio|SetSound _audio "/Game/Sounds/SQ_ThunderLoop.SQ_ThunderLoop")
  (Components|Activation|Activate _audio false))

(event Collision|EventActorBeginOverlap
  (params (OtherActor :type Actor%20Object%20Reference))
  (|CallParentFunction OtherActor) ; This node is disabled and will not be called.\nDrag off pins to build functionality.
)

(event EventTick
  (params (DeltaSeconds :type Float%20%28single-precision%29))
  (|CallParentFunction DeltaSeconds) ; This node is disabled and will not be called.\nDrag off pins to build functionality.
)

(fn ConstructionScript
  (|CallParentFunction))

(fn ApplyDamage
  (params (DamagedActor :type Actor%20Object%20Reference) (ImpactLocationIn :type Vector :default "0, 0, 0"))
  (|CallParentFunction DamagedActor ImpactLocationIn)
  (CallFunction|SpawnEmitter ImpactLocationIn))