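; BP_Wizard is an enemy that turns to face the VR player and fires projectiles at them.
; BeginPlay caches the MotionControllerPawn, and Tick sets the wizard's yaw toward that pawn's camera from its FiringPoint.
; A Delay on the Tick chain throttles firing to about every three seconds, spawning a scaled-down BP_EnemyProjectile at FiringPoint along the actor's rotation.
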(event EventBeginPlay
  ;[1 1 1] Player Reference Getter
  (bind _asmotion_controller_pawn (Utilities|Casting|CastToMotionControllerPawn (Game|Player|GetPlayerPawn 0)))
  (Variables|Default|SetPlayerReference _asmotion_controller_pawn))

(event Collision|EventActorBeginOverlap
  (params (OtherActor :type Actor%20Object%20Reference)))

(event EventTick
  (params (DeltaSeconds :type Float%20%28single-precision%29))
  ;[1 1 1] Enemy Rotation Controller
  (Transformation|SetActorRotation (Math|Rotator|MakeRotator 0.0 0.0 (.yaw (Math|Rotator|FindLookatRotation (Transformation|GetWorldLocation (Variables|Default|GetFiringPoint)) (Transformation|GetWorldLocation (Variables|/Game/VirtualRealityBP/Blueprints/MotionControllerPawn.MotionControllerPawn_C|GetCamera (Variables|Default|GetPlayerReference)))))))
  (Utilities|FlowControl|Delay 3.0)
  (Game|SpawnActorfromClass "/Game/BP_EnemyProjectile.BP_EnemyProjectile_C" (Math|Transform|MakeTransform (Transformation|GetWorldLocation (Variables|Default|GetFiringPoint)) (Transformation|GetActorRotation) "0.200000,0.200000,0.200000") "Undefined" self 0))

(fn ConstructionScript
  (|CallParentFunction))