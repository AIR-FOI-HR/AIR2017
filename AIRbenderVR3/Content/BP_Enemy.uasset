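; Enemy character Blueprint that handles health and death, in a game played through a MotionController pawn.
; AnyDamage subtracts from HP, and at zero or below it flags IsDead, calls Dead on its AIC_EnemyControler, updates score UI on MotionControllerPawn actors and destroys itself after a delay.
; The death branch has no repeat guard and stops if the controller cast fails.
; UpdateWalkSpeed exposes a setter for movement speed.
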(event Game|Damage|EventAnyDamage
  (params (Damage :type Float%20%28single-precision%29) (DamageType :type Damage%20Type%20Object%20Reference) (InstigatedBy :type Controller%20Object%20Reference) (DamageCauser :type Actor%20Object%20Reference))
  ;[1 1 1] Enemy Health Handler
  (Variables|Default|SetHP (- (Variables|Default|GetHP) Damage))
  (if (<= (Variables|Default|GetHP) 0.0)
    (Variables|Default|SetIsDead true)
    ;[1 1 1] Send Death Info
    (bind _asaic_enemy_controler (Utilities|Casting|CastToAIC_EnemyControler (Pawn|GetController)))
    (Default|Dead _asaic_enemy_controler)
    ;[1 1 1] Update UI
    (bind _outactors (Actor|GetAllActorsOfClass "/Game/VirtualRealityBP/Blueprints/MotionControllerPawn.MotionControllerPawn_C"))
    (Default|UpdateScoreNoUI _outactors)
    ;[1 1 1] Destroy Actor
    (Utilities|FlowControl|Delay 5.0)
    (Actor|DestroyActor)))

(fn ConstructionScript)

(fn UpdateWalkSpeed
  (params (NewWalkSpeed :type Float%20%28single-precision%29))
  (Variables|/Script/Engine.CharacterMovementComponent|SetMaxWalkSpeed (Variables|Character|GetCharacterMovement) NewWalkSpeed))