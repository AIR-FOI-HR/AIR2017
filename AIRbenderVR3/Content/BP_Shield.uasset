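; BP_Shield is a temporary rock shield actor that absorbs damage until it breaks or expires.
; BeginPlay plays an emerge sound and spray effect, adds a fire charge effect after a short delay, then destroys the shield after about five seconds if it still has health.
; AnyDamage subtracts from ShieldHealth and, at zero, destroys it with the same break particles and sound, played louder than on timeout.
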(event EventBeginPlay
  (bind _returnvalue (Transformation|GetActorLocation))
  (bind _returnvalue_2 (Transformation|GetActorLocation))
  (bind _returnvalue_3 (Transformation|GetActorLocation))
  (Audio|PlaySoundatLocation "/Game/Sounds/A_RockEmerge.A_RockEmerge" _returnvalue "0, 0, 0" 1.0 1.0 0.0 0 0 0)
  (Effects|SpawnEmitteratLocation "/Game/InfinityBladeEffects/Effects/FX_Mobile/combat/P_MagicSpray_Untyped.P_MagicSpray_Untyped" _returnvalue "90.000000, 0, 0" "0.700000,0.700000,0.700000")
  (Utilities|FlowControl|Delay 0.75)
  (Effects|SpawnEmitteratLocation "/Game/InfinityBladeEffects/Effects/FX_Mobile/Fire/combat/P_HeldCharge_Fire_01.P_HeldCharge_Fire_01" (Math|Vector|MakeVector (.x _returnvalue_3) (.y _returnvalue_3) (+ (.z _returnvalue_3) 3e+01)) (Transformation|GetActorRotation) "0.500000,0.500000,0.500000")
  (Utilities|FlowControl|Delay 4.25)
  (if (> (Variables|Default|GetShieldHealth) 0.0)
    (Effects|SpawnEmitteratLocation "/Game/InfinityBladeEffects/Effects/FX_Combat_Base/WeaponCombo/P_Cube_Mesh_Test.P_Cube_Mesh_Test" (Math|Vector|MakeVector (.x _returnvalue_2) (.y _returnvalue_2) (- (.z _returnvalue_2) 35.0)) "0, 0, 0" "0.500000,0.500000,0.500000")
    (Audio|PlaySoundatLocation "/Game/Sounds/A_RockBreak.A_RockBreak" (Transformation|GetActorLocation) "0, 0, 0" 0.5 1.0 0.0 0 0 0)
    (Actor|DestroyActor)))

(event Collision|EventActorBeginOverlap
  (params (OtherActor :type Actor%20Object%20Reference)))

(event EventTick
  (params (DeltaSeconds :type Float%20%28single-precision%29)))

(event Game|Damage|EventAnyDamage
  (params (Damage :type Float%20%28single-precision%29) (DamageType :type Damage%20Type%20Object%20Reference) (InstigatedBy :type Controller%20Object%20Reference) (DamageCauser :type Actor%20Object%20Reference))
  (bind _returnvalue (Transformation|GetActorLocation))
  (Variables|Default|SetShieldHealth (- (Variables|Default|GetShieldHealth) Damage))
  (if (<= (Variables|Default|GetShieldHealth) 0.0)
    (Effects|SpawnEmitteratLocation "/Game/InfinityBladeEffects/Effects/FX_Combat_Base/WeaponCombo/P_Cube_Mesh_Test.P_Cube_Mesh_Test" (Math|Vector|MakeVector (.x _returnvalue) (.y _returnvalue) (- (.z _returnvalue) 35.0)) "0, 0, 0" "0.500000,0.500000,0.500000")
    (Audio|PlaySoundatLocation "/Game/Sounds/A_RockBreak.A_RockBreak" (Transformation|GetActorLocation) "0, 0, 0" 0.5 1.0 0.0 0 0 0)
    (Actor|DestroyActor)))

(fn ConstructionScript)