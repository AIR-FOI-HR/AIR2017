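; Ice projectile Blueprint that adds looping flight audio and impact effects to its parent projectile class.
; BeginPlay starts the ice loop sound, and the ApplyDamage override runs the parent's damage logic before calling SpawnEmitter.
; SpawnEmitter plays an ice split particle, a raised, enlarged rock impact particle and an attenuated hit sound, then stops the loop and destroys the actor.
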(event Custom|Spawn%20Emitter
  (params (Impact%20Location :type Vector))
  (bind (_x _y _z) (Math|Vector|BreakVector Impact%20Location))
  (Effects|SpawnEmitteratLocation "/Game/InfinityBladeEffects/Effects/FX_Monsters/FX_Monster_Elemental/ICE/P_IceElementalSplit_Small.P_IceElementalSplit_Small" Impact%20Location)
  (Effects|SpawnEmitteratLocation "/Game/InfinityBladeEffects/Effects/FX_Treasure/Resources/P_Resource_Impact_Rock.P_Resource_Impact_Rock" (Math|Vector|MakeVector _x _y (+ _z 5e+01)) "0, 0, 0" "2.000000,2.000000,2.000000")
  (Audio|PlaySoundatLocation "/Game/Sounds/A_IceHit.A_IceHit" Impact%20Location "0, 0, 0" 0.8 1.0 0.0 "/Game/Sounds/SA_Explosion.SA_Explosion" 0 0)
  (Components|Activation|Deactivate (Variables|Default|GetAudio))
  (Actor|DestroyActor))

(event EventBeginPlay
  (bind _audio (Variables|Default|GetAudio))
  (|CallParentFunction)
  (Audio|Components|Audio|SetSound _audio "/Game/Sounds/SQ_IceLoop.SQ_IceLoop")
  (Components|Activation|Activate _audio false))

(event Collision|EventActorBeginOverlap
  (params (OtherActor :type Actor%20Object%20Reference))
  (|CallParentFunction OtherActor) ; This node is disabled and will not be called.\nDrag off pins to build functionality.
)

(event EventTick
  (params (DeltaSeconds :type Float%20%28single-precision%29))
  (|CallParentFunction DeltaSeconds) ; This node is disabled and will not be called.\nDrag off pins to build functionality.
)

(fn ConstructionScript
  (|CallParentFunction))

(fn ApplyDamage
  (params (DamagedActor :type Actor%20Object%20Reference) (ImpactLocationIn :type Vector :default "0, 0, 0"))
  (|CallParentFunction DamagedActor ImpactLocationIn)
  (CallFunction|SpawnEmitter ImpactLocationIn))