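; BP_TriggerArea is an actor that spawns and clears a set of BP_TrainingSphere actors at marked positions.
; CreateTrainingSpheres spawns a scaled-down sphere at the world location of each direct child component of TriggerAreaBox and stores it in the TrainingSpheres array.
; DestroyTrainingSpheres walks that array in reverse, destroying and removing each sphere.
; Both are custom events with no caller in this graph, as BeginPlay, overlap and Tick are disabled.
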(event Custom|CreateTrainingSpheres
  (for _array_element (Components|GetChildrenComponents (Variables|Default|GetTriggerAreaBox) false)
    (bind _returnvalue (Game|SpawnActorfromClass "/Game/BP_TrainingSphere.BP_TrainingSphere_C" (Math|Transform|MakeTransform (Transformation|GetWorldLocation _array_element) "0, 0, 0" "0.300000,0.300000,0.300000") "Undefined" 0 0))
    (Utilities|Array|Add (Variables|Default|GetTrainingSpheres) _returnvalue)))

(event Custom|DestroyTrainingSpheres
  (bind _trainingspheres (Variables|Default|GetTrainingSpheres))
  (bind _arrayelement (Utilities|Array|ReverseforEachLoop _trainingspheres)
    (:LoopBody
      (Actor|DestroyActor _arrayelement)
      (Utilities|Array|RemoveItem _trainingspheres _arrayelement))))

(event EventBeginPlay)

(event Collision|EventActorBeginOverlap
  (params (OtherActor :type Actor%20Object%20Reference)))

(event EventTick
  (params (DeltaSeconds :type Float%20%28single-precision%29)))

(fn ConstructionScript)