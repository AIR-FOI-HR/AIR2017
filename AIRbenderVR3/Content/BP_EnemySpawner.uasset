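; BP_EnemySpawner is an enemy spawner that periodically adds random enemy types within its SpawnerArea box.
; A looping timer started at BeginPlay spawns one AI pawn running BT_Enemy whenever the world's BP_Enemy count is below NumberOfEnemies.
; The NumberOfEnemies graph holds a difficulty-scaled logarithm of time since the last reset.
; ResetSpawner re-sets the timer and records that reset time.
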(event Custom|Spawn%20Enemies
  (bind _spawnerarea (Variables|Default|GetSpawnerArea))
  (bind _enemies (Variables|Default|GetEnemies))
  (bind _outactors (Actor|GetAllActorsOfClass "/Game/BP_Enemy.BP_Enemy_C"))
  (if (< (Utilities|Array|Length _outactors) (Utilities|NumberOfEnemies (Variables|Default|GetDifficulty)))
    (AI|SpawnAIFromClass (Utilities|Array|Get(acopy) _enemies (Math|Random|RandomInteger (Utilities|Array|Length _enemies))) "/Game/ThirdPersonBP/AI/BT_Enemy.BT_Enemy" (Math|Random|RandomPointinBoundingBox (Transformation|GetWorldLocation _spawnerarea) (Components|Box|GetScaledBoxExtent _spawnerarea)) "0, 0, 0" false 0)))

(event Custom|StartSpawner
  (bind _returnvalue (Utilities|Time|SetTimerbyFunctionName 0 "Spawn Enemies" (Variables|Default|GetSpawn%20interval) true))
  (Variables|Default|SetTimer _returnvalue))

(event Custom|ResetSpawner
  (bind _returnvalue (Utilities|Time|SetTimerbyFunctionName 0 "Spawn Enemies" (Variables|Default|GetSpawn%20interval) true))
  (Variables|Default|SetTimer _returnvalue)
  (Variables|Default|SetTime (Utilities|Time|GetGameTimeinSeconds)))

(event Collision|EventActorBeginOverlap
  (params (OtherActor :type Actor%20Object%20Reference)))

(event EventTick
  (params (DeltaSeconds :type Float%20%28single-precision%29)))

(event EventBeginPlay
  (CallFunction|StartSpawner))

(fn ConstructionScript)